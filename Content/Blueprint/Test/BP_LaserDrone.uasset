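; Test laser drone actor that turns to face the nearest BP_Lancer and aims a Niagara beam at it.
; Every Tick, SetupLaserEndPoint searches all BP_Lancer actors, writes the nearest one's location to BeamEndW and returns it for the look-at rotation.
; While ActivateLaser is true, Tick also activates the Niagara component; nothing here deactivates it.
; SetupEndLaserPoint repeats the beam endpoint logic but is not called from the event graph.
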(event EventBeginPlay)

(event Collision|EventActorBeginOverlap
  (params (OtherActor :type Actor%20Object%20Reference)))

(event EventTick
  (params (DeltaSeconds :type Float%20%28single-precision%29))
  (bind _returnvalue (Transformation|GetActorLocation))
  (bind _returnvalue_2 (CallFunction|SetupLaserEndPoint))
  (Transformation|SetActorLocationAndRotation _returnvalue (Math|Rotator|FindLookatRotation _returnvalue _returnvalue_2))
  (if (Variables|UserDefined|GetActivateLaser)
    (Components|Activation|Activate (Variables|Default|GetNiagara) false)))

(fn ConstructionScript)

(fn SetupLaserEndPoint
  (bind _outactors (Actor|GetAllActorsOfClass "/Game/Blueprint/Units/Lancer/BP_Lancer.BP_Lancer_C"))
  (Niagara|SetNiagaraVariable(Vector3) (Variables|Default|GetNiagara) "BeamEndW" (Transformation|GetActorLocation (.ReturnValue (Actor|FindNearestActor (Transformation|GetActorLocation) _outactors))))
  (return (Transformation|GetActorLocation (.ReturnValue (Actor|FindNearestActor (Transformation|GetActorLocation) _outactors)))))