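; Test actor that moves a sphere under the mouse cursor, snapped to a grid on a horizontal plane.
; BeginPlay shows the cursor and enables mouse-over events, and the Plane's cursor-over events toggle a hover flag.
; While hovered, Tick intersects the deprojected mouse ray with the plane, rounds X and Y to CellSize, and teleports the Sphere there.
; The click handler is empty.
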(event OnBeginCursorOver(Plane)
  (params (TouchedComponent :type Primitive%20Component%20Object%20Reference))
  (Variables|Default|SetisMouseHover true))

(event OnEndCursorOver(Plane)
  (params (TouchedComponent :type Primitive%20Component%20Object%20Reference))
  (Variables|Default|SetisMouseHover false))

(event OnClicked(Plane)
  (params (TouchedComponent :type Primitive%20Component%20Object%20Reference) (ButtonPressed :type Key%20Structure)))

(event EventBeginPlay
  (bind _returnvalue (Game|GetPlayerController 0))
  (Variables|/Script/Engine.PlayerController|SetbEnableMouseOverEvents _returnvalue true)
  (Variables|/Script/Engine.PlayerController|SetbShowMouseCursor _returnvalue true))

(event EventTick
  (params (DeltaSeconds :type Float%20%28single-precision%29))
  (bind _cellsize (Variables|Default|GetCellSize))
  (if (Variables|Default|GetisMouseHover)
    (bind _intersection (CallFunction|GetPointonPlane))
    (bind _returnvalue (CallFunction|SnaptoGrid (.x _intersection) _cellsize))
    (bind _returnvalue_2 (CallFunction|SnaptoGrid (.y _intersection) _cellsize))
    (Transformation|SetWorldLocation (Variables|Default|GetSphere) (Math|Vector|MakeVector _returnvalue _returnvalue_2 (.z _intersection)) false true)))

(fn ConstructionScript)

(fn GetPointonPlane
  (bind _returnvalue (Game|GetPlayerController 0))
  (bind (_worldlocation _worlddirection) (Game|Player|ConvertMouseLocationToWorldSpace _returnvalue))
  (return (.Intersection (Class|KismetMathLibrary|LinePlaneIntersectionOriginNormal _worldlocation (+ _worldlocation (* _worlddirection 1e+04)) (Transformation|GetWorldLocation (Variables|Default|GetPlane)) "0.000000,0.000000,1.000000"))))

(fn SnaptoGrid
  (params (A :type Float%20%28double-precision%29) (GridCell :type Float%20%28double-precision%29))
  (return (Math|Conversions|ToFloat(Integer) (* (Class|KismetMathLibrary|Round64 (/ A GridCell)) (Class|KismetMathLibrary|ToInt64(Float) GridCell)))))